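; BP_InsertionSort is an algorithm Blueprint that implements insertion sort on its Array variable, alongside helpers to append numbers and print each index and value.
; InsertionSortAlgorithm walks each element backward, swapping it with its left neighbor when smaller, producing ascending order in place.
; The inner loop has no early exit, so it always scans down to index zero.
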(fn `AddNumber`
  (params (NewNumber :type Integer))
  (`KismetArrayLibrary.Array_Add` (`self.Array`) NewNumber)
  (return))

(fn `InsertionSortAlgorithm`
  (locals (TempIndex :type Integer))
  (bind _tempindex (`local.TempIndex`))
  (set `local.TempIndex` 0)
  (for _index (range 1 (+ (`KismetArrayLibrary.Array_LastIndex` (`self.Array`)) 1))
    (set `local.TempIndex` _index)
    (while (> (`local.TempIndex`) 0)
      (if (< (`|GetArrayItem` (`self.Array`) (`local.TempIndex`)) (`|GetArrayItem` (`self.Array`) (- (`local.TempIndex`) 1)))
        (`KismetArrayLibrary.Array_Swap` (`self.Array`) _tempindex (- _tempindex 1))
        (`/Engine/EditorBlueprintResources/StandardMacros.DecrementInt` (`local.TempIndex`))
        (else
          (`/Engine/EditorBlueprintResources/StandardMacros.DecrementInt` (`local.TempIndex`))))))
  (return))

(fn `PrintArray`
  (for (_array_element _array_index) (`self.Array`)
    (`KismetSystemLibrary.PrintString` null (`KismetStringLibrary.Concat_StrStr` (`KismetStringLibrary.Concat_StrStr` "Index: " (`KismetStringLibrary.Conv_IntToString` _array_index)) (`KismetStringLibrary.Concat_StrStr` "| Value: " (`KismetStringLibrary.Conv_IntToString` _array_element)))))
  (return))