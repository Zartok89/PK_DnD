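; BP_LinkedList is a singly linked list data structure in Blueprint, built from BP_Node_LL objects chained through Next references from a Head.
; Append walks to the tail to attach a new node, while Prepend swaps in a new Head.
; DeleteWithValue unlinks the first node with matching Data by re-pointing references.
; PrintList traverses from Head and prints each node's Data.
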(fn `Append`
  (params (Data :type String))
  (locals (mData :type String) (Current :type "/Game/PKDnD/DatastructureAndAlgorithms/LinkedList/BP_Node_LL Object Reference"))
  (set `local.mData` Data)
  (`/Engine/EditorBlueprintResources/StandardMacros.IsValid` (`self.Head`)
    (:`Is Valid`
      (set `local.Current` (`self.Head`))
      (while (`KismetSystemLibrary.IsValid` (`/Game/PKDnD/DatastructureAndAlgorithms/LinkedList/BP_Node_LL.Next` (`local.Current`)))
        (set `local.Current` (`/Game/PKDnD/DatastructureAndAlgorithms/LinkedList/BP_Node_LL.Next` (`local.Current`))))
      (bind _returnvalue (`|GenericCreateObject` "/Game/PKDnD/DatastructureAndAlgorithms/LinkedList/BP_Node_LL.BP_Node_LL_C"))
      (bind _reference (`/Game/PKDnD/DatastructureAndAlgorithms/LinkedList/BP_Node_LL.Node` _returnvalue (`local.mData`)))
      (set `/Game/PKDnD/DatastructureAndAlgorithms/LinkedList/BP_Node_LL.Next` _reference (`local.Current`))
      (return))
    (:`Is Not Valid`
      (bind _returnvalue_2 (`|GenericCreateObject` "/Game/PKDnD/DatastructureAndAlgorithms/LinkedList/BP_Node_LL.BP_Node_LL_C"))
      (bind _reference_2 (`/Game/PKDnD/DatastructureAndAlgorithms/LinkedList/BP_Node_LL.Node` _returnvalue_2 (`local.mData`)))
      (set `self.Head` _reference_2)
      (return))))

(fn `DeleteWithValue`
  (params (Data :type String))
  (locals (mData :type String) (Current :type "/Game/PKDnD/DatastructureAndAlgorithms/LinkedList/BP_Node_LL Object Reference"))
  (set `local.mData` Data)
  (`/Engine/EditorBlueprintResources/StandardMacros.IsValid` (`self.Head`)
    (:`Is Valid`
      (if (== (`/Game/PKDnD/DatastructureAndAlgorithms/LinkedList/BP_Node_LL.Data` (`self.Head`)) (`local.mData`))
        (if (`KismetSystemLibrary.IsValid` (`/Game/PKDnD/DatastructureAndAlgorithms/LinkedList/BP_Node_LL.Next` (`self.Head`)))
          (set `self.Head` (`/Game/PKDnD/DatastructureAndAlgorithms/LinkedList/BP_Node_LL.Next` (`self.Head`)))
          (return)
          (else
            (set `self.Head` null)
            (return)))
        (else
          (set `local.Current` (`self.Head`))
          (while (`KismetSystemLibrary.IsValid` (`/Game/PKDnD/DatastructureAndAlgorithms/LinkedList/BP_Node_LL.Next` (`local.Current`)))
            (if (== (`/Game/PKDnD/DatastructureAndAlgorithms/LinkedList/BP_Node_LL.Data` (`/Game/PKDnD/DatastructureAndAlgorithms/LinkedList/BP_Node_LL.Next` (`local.Current`))) (`local.mData`))
              (if (`KismetSystemLibrary.IsValid` (`/Game/PKDnD/DatastructureAndAlgorithms/LinkedList/BP_Node_LL.Next` (`/Game/PKDnD/DatastructureAndAlgorithms/LinkedList/BP_Node_LL.Next` (`local.Current`))))
                (set `/Game/PKDnD/DatastructureAndAlgorithms/LinkedList/BP_Node_LL.Next` (`/Game/PKDnD/DatastructureAndAlgorithms/LinkedList/BP_Node_LL.Next` (`/Game/PKDnD/DatastructureAndAlgorithms/LinkedList/BP_Node_LL.Next` (`local.Current`))) (`local.Current`))
                (return)
                (else
                  (set `/Game/PKDnD/DatastructureAndAlgorithms/LinkedList/BP_Node_LL.Next` null (`local.Current`))
                  (return)))
              (else
                (set `local.Current` (`/Game/PKDnD/DatastructureAndAlgorithms/LinkedList/BP_Node_LL.Next` (`local.Current`)))))))))
    (:`Is Not Valid`
      (return))))

(fn `Prepend`
  (params (Data :type String))
  (locals (mData :type String) (Current :type "/Game/PKDnD/DatastructureAndAlgorithms/LinkedList/BP_Node_LL Object Reference"))
  (set `local.mData` Data)
  (`/Engine/EditorBlueprintResources/StandardMacros.IsValid` (`self.Head`)
    (:`Is Valid`
      (bind _returnvalue (`|GenericCreateObject` "/Game/PKDnD/DatastructureAndAlgorithms/LinkedList/BP_Node_LL.BP_Node_LL_C"))
      (bind _reference (`/Game/PKDnD/DatastructureAndAlgorithms/LinkedList/BP_Node_LL.Node` _returnvalue (`local.mData`)))
      (bind _output_get (set `local.Current` _reference))
      (set `/Game/PKDnD/DatastructureAndAlgorithms/LinkedList/BP_Node_LL.Next` (`self.Head`) _output_get)
      (set `self.Head` (`local.Current`))
      (return))
    (:`Is Not Valid`
      (bind _returnvalue_2 (`|GenericCreateObject` "/Game/PKDnD/DatastructureAndAlgorithms/LinkedList/BP_Node_LL.BP_Node_LL_C"))
      (bind _reference_2 (`/Game/PKDnD/DatastructureAndAlgorithms/LinkedList/BP_Node_LL.Node` _returnvalue_2 (`local.mData`)))
      (set `self.Head` _reference_2)
      (return))))

(fn `PrintList`
  (locals (Current :type "/Game/PKDnD/DatastructureAndAlgorithms/LinkedList/BP_Node_LL Object Reference"))
  (`/Engine/EditorBlueprintResources/StandardMacros.IsValid` (`self.Head`)
    (:`Is Valid`
      (set `local.Current` (`self.Head`))
      (while (`KismetSystemLibrary.IsValid` (`local.Current`))
        (`KismetSystemLibrary.PrintString` null (`/Game/PKDnD/DatastructureAndAlgorithms/LinkedList/BP_Node_LL.Data` (`local.Current`)))
        (set `local.Current` (`/Game/PKDnD/DatastructureAndAlgorithms/LinkedList/BP_Node_LL.Next` (`local.Current`))))
      (return))
    (:`Is Not Valid`
      (return))))